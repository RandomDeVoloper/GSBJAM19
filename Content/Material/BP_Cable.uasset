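; BP_Cable is a cable actor that builds its mesh along an editable spline in the Construction Script, with no runtime logic.
; Each loop step adds two overlapping spline meshes from point Index to Index - 1, starting at 0 and skipping the last point, attached to CableComponent.
; The first mesh has no collision, gets a dynamic MAT_Cable_Edge material tinted by Color through PowerOn, and is stored in Components.
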(event EventBeginPlay)

(event Collision|EventActorBeginOverlap
  (params (OtherActor :type Actor%20Object%20Reference)))

(event EventTick
  (params (DeltaSeconds :type Float%20%28single-precision%29)))

(fn ConstructionScript
  (bind _spline (Variables|Default|GetSpline))
  (for _index (range 0 (- (Spline|GetNumberOfSplinePoints (Variables|Default|GetSpline)) 2))
    (bind _returnvalue (AddComponent|AddSplineMeshComponent false))
    (Collision|SetCollisionEnabled _returnvalue "NoCollision")
    (bind _returnvalue_2 (Rendering|Material|CreateDynamicMaterialInstance "/Game/Material/MAT_Cable_Edge.MAT_Cable_Edge" "None" "None" :!class /Script/Engine.KismetMaterialLibrary))
    (Rendering|Material|SetVectorParameterValue _returnvalue_2 "PowerOn" (Variables|Default|GetColor) :!class /Script/Engine.MaterialInstanceDynamic)
    (Rendering|Material|SetMaterial _returnvalue 0 _returnvalue_2)
    (Utilities|Array|Add (Variables|Default|GetComponents) _returnvalue)
    (Transformation|AttachComponentToComponent _returnvalue (Variables|Default|GetCableComponent) "None" "KeepRelative" "KeepRelative" "KeepRelative" true)
    (SplineMesh|SetStartandEnd _returnvalue (.Location (Spline|GetLocationandTangentatSplinePoint _spline _index "Local")) (.Tangent (Spline|GetLocationandTangentatSplinePoint _spline _index "Local")) (.Location (Spline|GetLocationandTangentatSplinePoint _spline (- _index 1) "Local")) (.Tangent (Spline|GetLocationandTangentatSplinePoint _spline (- _index 1) "Local")) true :!class /Script/Engine.SplineMeshComponent)
    (bind _returnvalue_3 (AddComponent|AddSplineMeshComponent false))
    (Transformation|AttachComponentToComponent _returnvalue_3 (Variables|Default|GetCableComponent) "None" "KeepRelative" "KeepRelative" "KeepRelative" true)
    (SplineMesh|SetStartandEnd _returnvalue_3 (.Location (Spline|GetLocationandTangentatSplinePoint _spline _index "Local")) (.Tangent (Spline|GetLocationandTangentatSplinePoint _spline _index "Local")) (.Location (Spline|GetLocationandTangentatSplinePoint _spline (- _index 1) "Local")) (.Tangent (Spline|GetLocationandTangentatSplinePoint _spline (- _index 1) "Local")) true :!class /Script/Engine.SplineMeshComponent)))