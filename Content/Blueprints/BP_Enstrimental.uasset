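; Orchestra instrument cable Blueprint that manages twelve cable references named after instruments, apparently for a cable-holding interaction with the player.
; BeginPlay caches the BP_Simsek player character, fills the cable array and zeroes the active cable's EndLocation.
; While CableHeld is set, Tick keeps zeroing that EndLocation after validity checks.
; CableHeld and ActiveCableIndex are only read here, never set.
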(event EventBeginPlay
  (bind _asbp_simsek (Utilities|Casting|CastToBP_Simsek (Game|GetPlayerCharacter 0)))
  (Variables|Default|SetPlayerRef _asbp_simsek)
  (bind _output_get (Variables|Default|SetArray (Utilities|Array|MakeArray (Variables|Default|GetKeman) (Variables|Default|Getkontrfagot) (Variables|Default|GetÇello) (Variables|Default|Getkontrbas) (Variables|Default|Gettrumpets) (Variables|Default|Getfrench%20horn) (Variables|Default|Gettrombone) (Variables|Default|Gettuba) (Variables|Default|Getyan%20flüt) (Variables|Default|Getobua) (Variables|Default|Getfagot) (Variables|Default|GetViyola))))
  (Variables|/Script/CableComponent.CableComponent|SetEndLocation (Utilities|Array|Get(acopy) _output_get (Variables|Default|GetActiveCableIndex)) (Math|Vector|MakeVector 0.0 0.0 0.0)))

(event EventTick
  (params (DeltaSeconds :type Float%20%28single-precision%29))
  (bind _array (Variables|Default|GetArray))
  (bind _activecableindex (Variables|Default|GetActiveCableIndex))
  (bind _output (Utilities|Array|Get(acopy) _array _activecableindex))
  (if (Variables|Default|GetbCableHeld)
    (Utilities|IsValid (Variables|Default|GetPlayerRef)
      (:Is%20Valid
        (Utilities|IsValid _output
          (:Is%20Valid
            (Variables|/Script/CableComponent.CableComponent|SetEndLocation _output (Math|Vector|MakeVector 0.0 0.0 0.0))))))))

(fn ConstructionScript)