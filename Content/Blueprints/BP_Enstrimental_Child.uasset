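; BP_Enstrimental_Child is a child Blueprint that supplies a set of orchestral instrument sounds, spanning strings, brass, woodwinds and harpsichord.
; BeginPlay fills the Sounds array in a fixed order without calling the parent's BeginPlay.
; The graph holds no playback logic, Tick and overlap are disabled stubs, and the Bozuk node is unused.
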(event Collision|EventActorBeginOverlap
  (params (OtherActor :type Actor%20Object%20Reference)))

(event EventTick
  (params (DeltaSeconds :type Float%20%28single-precision%29))
  (|CallParentFunction DeltaSeconds) ; This node is disabled and will not be called.\nDrag off pins to build functionality.
)

(event EventBeginPlay
  (Variables|Default|SetSounds (Utilities|Array|MakeArray (Variables|Default|GetKeman-1) (Variables|Default|GetViyola1) (Variables|Default|GetKeman-2) (Variables|Default|GetTrombones) (Variables|Default|GetTrumpets1) (Variables|Default|GetFrench_Horn) (Variables|Default|GetTuba1) (Variables|Default|GetBass_0) (Variables|Default|GetFlüt_0) (Variables|Default|GetObua1) (Variables|Default|GetFagot1_0) (Variables|Default|GetKlavsen))))

(fn ConstructionScript
  (|CallParentFunction))